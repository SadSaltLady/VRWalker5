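; BP_Data is an actor that acts as a socket client for sending string data to a configured IP and port.
; It connects on BeginPlay or through the Reconnect event, stores the connection ID when connected, and disconnects when destroyed.
; TransmitData converts a string to bytes and sends it over that connection.
; The disconnect and message-received callbacks are empty, so incoming data is ignored and reconnection is not automatic.
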(event `Reconnect`
  (`self.Connect` (`self.IP`) (`self.Port`) (`|CreateDelegate` :!event `On Disconnected`) (`|CreateDelegate` :!event `On Connected`) (`|CreateDelegate` :!event `On Message Received`) :!label _label))

(event `self.ReceiveBeginPlay`
  (goto _label))

(event `self.ReceiveDestroyed`
  (`self.Disconnect` (`self.Connection Id`)))

(fn `On Connected`
  (params (ConnectionId :type Integer))
  (set `self.Connection Id` ConnectionId))

(fn `On Disconnected`
  (params (ConnectionId :type Integer)))

(fn `On Message Received`
  (params (ConnectionId :type Integer) (Message :type "Array of Byte (by ref)"))
  (return))

(fn `TransmitData`
  (params (String :type String))
  (`self.SendData` (`self.Connection Id`) (`self.Conv_StringToBytes` String)))

(fn `UserConstructionScript`)