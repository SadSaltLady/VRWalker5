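; Runs a VR study procedure that logs participant movement across situations switching between high-res, low-res and box lab visuals.
; Three controller samples from VRPawn dispatchers align the scene root to calibration markers and define local space for logged positions.
; Once readied, leaving the EndDetection volume starts recording and re-entering stops it, with an indicator color showing state.
; A looping timer drives sampling, and DataTransmitter sends CSV motion and waypoint data.
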(event `self.ReceiveBeginPlay`
  (`|ExecutionSequence`
    (:`then_0`
      (`SceneComponent.SetVisibility` (`self.Lab_lowrez`) false true)
      ;[1 1 1] Set Partcipant ID
      (bind _output_get (set `self.ParticipantID` (`KismetMathLibrary.RandomIntegerInRange` 0 100)))
      (`KismetSystemLibrary.PrintString` (`KismetStringLibrary.Concat_StrStr` "Particpant ID is: " (`KismetStringLibrary.Conv_IntToString` _output_get)) true true (struct :`R` 1.0 :`G` 0.047428 :`A` 1.0) 20.0))
    (:`then_1`
      ;[1 1 1] Setting Reference to Player Pawn
      (bind _asvrpawn (cast `/Game/VRTemplate/Blueprints/VRPawn` (`Controller.K2_GetPawn` (`GameplayStatics.GetPlayerController` 0)))
        (:`then`
          (set `self.VRPawnRef` _asvrpawn)
          ;[1 1 1] Bind Event Dispatchers to our events
          (add `/Game/VRTemplate/Blueprints/VRPawn.SendCalibrationInfo` (`self.VRPawnRef`) (`|CreateDelegate` :!event `RecordCalibrationData`))
          (add `/Game/VRTemplate/Blueprints/VRPawn.StartRecordingSession` (`self.VRPawnRef`) (`|CreateDelegate` :!event `StartRecordingSession`))
          (add `/Game/VRTemplate/Blueprints/VRPawn.EndRecordingSession` (`self.VRPawnRef`) (`|CreateDelegate` :!event `EndRecordingSession`))
          (add `/Game/VRTemplate/Blueprints/VRPawn.ReadyForNext` (`self.VRPawnRef`) (`|CreateDelegate` :!event `ReadyForNextSession`)))
        (:`CastFailed`
          (`KismetSystemLibrary.PrintString` "In BP_MainProcedure, Cast to VR Pawn failed"))))))

(event `StartRecordingSession`
  ;[0.5121 1 0.3254] Handle Recording Logistics
  ;;[1 1 1] Start Recording Session
  (`/Game/_Blueprints/BP_Data.TransmitData` (`self.DataTransmitter`) "start")
  (`/Game/_Blueprints/BP_Data.TransmitData` (`self.DataTransmitter`) (`self.MakeFilename` "Data"))
  (bind _returnvalue (`KismetSystemLibrary.K2_SetTimerDelegate` (`|CreateDelegate` :!event `Record`) 0.125 true)) ; original time value of 0.03125
  (set `self.RecorderTimer` _returnvalue))

(event `RecordCalibrationData`
  (params (RightControllerLoc :type "Vector Structure"))
  ;[0.5121 1 0.3254] Handle Recording Logistics
  ;;[1 1 1] Recording and executing on calibration data
  (if (== (`self.CalibrationCount`) 3)
    (`self.Calibrate`)
    (set `self.CalibrationCount` 0)
    (else
      ;;;[0.1476 0.269 1] record 3 data points in order
      (`KismetArrayLibrary.Array_Set` (`self.CalibrationDatapoints`) (`self.CalibrationCount`) RightControllerLoc true)
      (`/Engine/EditorBlueprintResources/StandardMacros.IncrementInt` (`self.CalibrationCount`)
        (:`  `
          (`KismetSystemLibrary.PrintString` "RECRODING"))))))

(event `self.EndDetection.OnComponentBeginOverlap`
  (params (OverlappedComponent :type "PrimitiveComponent Object Reference") (OtherActor :type "Actor Object Reference") (OtherComp :type "PrimitiveComponent Object Reference") (OtherBodyIndex :type Integer) (bFromSweep :type Boolean) (SweepResult :type "HitResult Structure (by ref)"))
  ;[1 1 1 1 30] User Overallaped EndDetection
  (cast `/Game/VRTemplate/Blueprints/VRPawn` OtherActor
    (:`then`
      (if (`self.Recording`)
        ;;[1 1 1] end recording
        (set `self.Recording` false)
        (`self.EndRecordingSession`)
        (`MaterialInstanceDynamic.SetVectorParameterValue` (`self.MatieralIndicator`) "Color" (struct :`R` 0.958333 :`G` 0.958333 :`B` 0.958333 :`A` 1.0))
        (`KismetSystemLibrary.PrintString` "ENDDDDDDDDDDDDDDDDDDDDDDDDDDDDDDDDDDDDDDD" true true (struct :`G` 0.66 :`B` 1.0 :`A` 1.0) 5.0)
        (set `self.WaypointData` "")))
    (:`CastFailed`
      (`KismetSystemLibrary.PrintString` "EndDetection failed to overlap with VRPawn :(" :!label _label))))

(event `EndRecordingSession`
  ;[0.5121 1 0.3254] Handle Recording Logistics
  ;;[1 1 1] End Recording Session
  (`KismetSystemLibrary.K2_ClearAndInvalidateTimerHandle` (`self.RecorderTimer`))
  (`/Game/_Blueprints/BP_Data.TransmitData` (`self.DataTransmitter`) (`self.WaypointData`))
  (`/Game/_Blueprints/BP_Data.TransmitData` (`self.DataTransmitter`) "stop"))

(event `self.EndDetection.OnComponentEndOverlap`
  (params (OverlappedComponent :type "PrimitiveComponent Object Reference") (OtherActor :type "Actor Object Reference") (OtherComp :type "PrimitiveComponent Object Reference") (OtherBodyIndex :type Integer))
  ;[1 1 1 1 30] User Overallaped EndDetection
  (cast `/Game/VRTemplate/Blueprints/VRPawn` OtherActor
    (:`then`
      (if (`self.ReadyToRecord`)
        ;;[1 1 1] start recording
        (set `self.Recording` true)
        (set `self.ReadyToRecord` false)
        (`self.StartRecordingSession`)
        (`MaterialInstanceDynamic.SetVectorParameterValue` (`self.MatieralIndicator`) "Color" (struct :`G` 0.552832 :`B` 0.958333 :`A` 1.0))
        (`KismetSystemLibrary.PrintString` "SSSSSSSTTTTTTTTARRRRRRRRRRT" true true (struct :`R` 1.0 :`B` 0.563425 :`A` 1.0) 5.0)))
    (:`CastFailed`
      (goto _label))))

(event `ReadyForNextSession`
  ;[0.5121 1 0.3254] Handle Recording Logistics
  ;;[1 1 1] Comment
  (`KismetSystemLibrary.PrintString` "He----------------------------------------------------llo")
  (set `self.ReadyToRecord` true)
  (`self.ResetTouchpoint`)
  (switch `int` (mod (`self.SituationID`) 4)
    (:`Default`
      _)
    (:`0`
      _)
    (:`1`
      ;;;[1 1 1] VirtualScan
      (`SceneComponent.SetVisibility` (`self.Lab_Highrez`) true false)
      (`SceneComponent.SetVisibility` (`self.Lab_lowrez`) false false)
      (`SceneComponent.SetVisibility` (`self.Lab_Box`) false false))
    (:`2`
      ;;;[1 1 1] Demo Reality
      (`SceneComponent.SetVisibility` (`self.Lab_Highrez`) false false)
      (`SceneComponent.SetVisibility` (`self.Lab_lowrez`) true false)
      (`SceneComponent.SetVisibility` (`self.Lab_Box`) false false))
    (:`3`
      ;;;[1 1 1] Box Reality
      (`SceneComponent.SetVisibility` (`self.Lab_Highrez`) false false)
      (`SceneComponent.SetVisibility` (`self.Lab_lowrez`) false false)
      (`SceneComponent.SetVisibility` (`self.Lab_Box`) true false)))
  (`MaterialInstanceDynamic.SetVectorParameterValue` (`self.MatieralIndicator`) "Color" (struct :`R` 0.958333 :`G` 0.120984 :`A` 1.0))
  (`/Engine/EditorBlueprintResources/StandardMacros.IncrementInt` (`self.SituationID`)))

(fn `Calibrate`
  (`SceneComponent.K2_SetWorldRotation` (`self.DefaultSceneRoot`) (`SmoothConverters.CalculateRotation` (`self.CalibrationDatapoints`)) false false)
  (`SceneComponent.K2_AddWorldOffset` (`self.DefaultSceneRoot`) (`SmoothConverters.CalculateOffset` (`self.CalibrationDatapoints`) (`SceneComponent.K2_GetComponentLocation` (`self.Calibration1`)) (`SceneComponent.K2_GetComponentLocation` (`self.Calibration2`)) (`SceneComponent.K2_GetComponentLocation` (`self.Calibration3`))) false false)
  (set `self.LocalSpaceTransform` (`KismetMathLibrary.InvertTransform` (`SceneComponent.K2_GetComponentToWorld` (`self.DefaultSceneRoot`))))
  (`SceneComponent.SetVisibility` (`self.Calibration3`) false false)
  (`SceneComponent.SetVisibility` (`self.Calibration2`) false false)
  (`SceneComponent.SetVisibility` (`self.Calibration1`) false false))

(fn `DataCollecting`)

(fn `DataToCSV`
  (params (Data :type "_Data Structure"))
  (returns (PrettyData :type String))
  (bind (_time _headpos _controllerleftpos _controllerrightpos _angularacceleration _linearacceleration _angularvelocity _linearvelocity) (break `_Data` Data))
  (return (`KismetStringLibrary.Concat_StrStr` (`KismetStringLibrary.Conv_DoubleToString` _time) "," (`SmoothConverters.VectorToNiceString` _headpos) "," (`SmoothConverters.VectorToNiceString` _controllerleftpos) "," (`SmoothConverters.VectorToNiceString` _controllerrightpos) "," (`SmoothConverters.VectorToNiceString` _angularacceleration) "," (`SmoothConverters.VectorToNiceString` _linearacceleration) "," (`SmoothConverters.VectorToNiceString` _angularvelocity) "," (`SmoothConverters.VectorToNiceString` _linearvelocity))))

(fn `DumpToStruct`
  (returns (Data :type "_Data Structure"))
  (bind _vrpawnref (`self.VRPawnRef`))
  (bind _localspacetransform (`self.LocalSpaceTransform`))
  (bind (_headpos _controllerleftpos _controllerrightpos) (`/Game/VRTemplate/Blueprints/VRPawn.GetEverythingData` _vrpawnref))
  (bind (_time_seconds_ _angularacceleration _linearacceleration _angularvelocity _linearvelocity) (`/Game/VRTemplate/Blueprints/VRPawn.GetMovementData` _vrpawnref))
  (return (make `_Data` _time_seconds_ (`KismetMathLibrary.TransformLocation` _localspacetransform _headpos) (`KismetMathLibrary.TransformLocation` _localspacetransform _controllerleftpos) (`KismetMathLibrary.TransformLocation` _localspacetransform _controllerrightpos) _angularacceleration _linearacceleration _angularvelocity _linearvelocity)))

(fn `MakeFilename`
  (params (SetName :type String))
  (returns (filename :type String))
  (return (`KismetStringLibrary.Concat_StrStr` (`KismetStringLibrary.Conv_IntToString` (`self.ParticipantID`)) "_situa" (`KismetStringLibrary.Conv_IntToString` (`self.SituationID`)) "_" SetName ".csv")))

(fn `Record`
  (bind _data (`self.DumpToStruct`))
  (bind _prettydata (`self.DataToCSV` _data))
  (`/Game/_Blueprints/BP_Data.TransmitData` (`self.DataTransmitter`) _prettydata))

(fn `RecordWaypoints`
  (params (ID :type Text))
  (set `self.WaypointData` (`KismetStringLibrary.Concat_StrStr` (`self.WaypointData`) (`KismetTextLibrary.Conv_TextToString` ID) "," (`KismetStringLibrary.Conv_DoubleToString` (`KismetSystemLibrary.GetGameTimeInSeconds`)) ",")))

(fn `ResetTouchPoints`)

(fn `SaveData`
  (`|ExecutionSequence`
    (:`then_0`
      (`/Game/_Blueprints/BP_Data.TransmitData` (`self.DataTransmitter`) (`self.FileData` "locations.csv" (`SmoothConverters.VectorArrToString` (`self.Locations`)))))
    (:`then_1`
      (`/Game/_Blueprints/BP_Data.TransmitData` (`self.DataTransmitter`) (`self.FileData` "velociacc.csv" (`SmoothConverters.VectorArrToString` (`self.VelocityAcc`)))))))

(fn `UserConstructionScript`
  (bind _startarea (`self.StartArea`))
  (bind _returnvalue (`PrimitiveComponent.CreateDynamicMaterialInstance` _startarea 0 null "None"))
  (`PrimitiveComponent.SetMaterial` _startarea 0 _returnvalue)
  (set `self.MatieralIndicator` _returnvalue))