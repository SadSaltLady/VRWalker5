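; Main procedure actor for a VR experiment that calibrates its placement and records participant movement per session.
; Three right-controller points from VRPawn events drive rotation and offset of the root against three calibration markers.
; Entering the EndDetection volume arms or stops recording and leaving it while armed starts recording, with a material color indicator.
; A looping timer samples the session, and DataTransmitter sends pawn tracking as CSV rows between start/stop messages.
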(event `self.ReceiveBeginPlay`
  (`|ExecutionSequence`
    (:`then_0`
      (`SceneComponent.SetVisibility` (`self.Lab_lowrez`) false true)
      ;[1 1 1] Set Partcipant ID
      (bind _output_get (set `self.ParticipantID` (`KismetMathLibrary.RandomIntegerInRange` 0 100)))
      (`KismetSystemLibrary.PrintString` (`KismetStringLibrary.Concat_StrStr` "Particpant ID is: " (`KismetStringLibrary.Conv_IntToString` _output_get)) true true (struct :`R` 1.0 :`G` 0.047428 :`A` 1.0) 20.0))
    (:`then_1`
      ;[1 1 1] Setting Reference to Player Pawn
      (bind _asvrpawn (cast `/Game/VRTemplate/Blueprints/VRPawn` (`Controller.K2_GetPawn` (`GameplayStatics.GetPlayerController` 0)))
        (:`then`
          (set `self.VRPawnRef` _asvrpawn)
          ;[1 1 1] Bind Event Dispatchers to our events
          (add `/Game/VRTemplate/Blueprints/VRPawn.SendCalibrationInfo` (`self.VRPawnRef`) (`|CreateDelegate` :!event `RecordCalibrationData`))
          (add `/Game/VRTemplate/Blueprints/VRPawn.StartRecordingSession` (`self.VRPawnRef`) (`|CreateDelegate` :!event `StartRecordingSession`))
          (add `/Game/VRTemplate/Blueprints/VRPawn.EndRecordingSession` (`self.VRPawnRef`) (`|CreateDelegate` :!event `EndRecordingSession`)))
        (:`CastFailed`
          (`KismetSystemLibrary.PrintString` "In BP_MainProcedure, Cast to VR Pawn failed"))))))

(event `StartRecordingSession`
  ;[0.5121 1 0.3254] Handle Recording Logistics
  ;;[1 1 1] Start Recording Session
  (`/Engine/EditorBlueprintResources/StandardMacros.IncrementInt` (`self.SituationID`)
    (:`  `
      (`/Game/_Blueprints/BP_Data.TransmitData` (`self.DataTransmitter`) "start")
      (`/Game/_Blueprints/BP_Data.TransmitData` (`self.DataTransmitter`) (`self.BuildFileName` "Experiment"))
      (`/Game/_Blueprints/BP_Data.TransmitData` (`self.DataTransmitter`) (`self.Header`))
      (bind _returnvalue (`KismetSystemLibrary.K2_SetTimerDelegate` (`|CreateDelegate` :!event `Record`) 0.1 true)) ; original time value of 0.03125
      (set `self.RecorderTimer` _returnvalue))))

(event `RecordCalibrationData`
  (params (RightControllerLoc :type "Vector Structure"))
  ;[0.5121 1 0.3254] Handle Recording Logistics
  ;;[1 1 1] Recording and executing on calibration data
  (if (== (`self.CalibrationCount`) 3)
    (`self.Calibrate`)
    (set `self.CalibrationCount` 0)
    (else
      ;;;[0.1476 0.269 1] record 3 data points in order
      (`KismetArrayLibrary.Array_Set` (`self.CalibrationDatapoints`) (`self.CalibrationCount`) RightControllerLoc true)
      (`/Engine/EditorBlueprintResources/StandardMacros.IncrementInt` (`self.CalibrationCount`)
        (:`  `
          (`KismetSystemLibrary.PrintString` "RECRODING"))))))

(event `self.EndDetection.OnComponentBeginOverlap`
  (params (OverlappedComponent :type "PrimitiveComponent Object Reference") (OtherActor :type "Actor Object Reference") (OtherComp :type "PrimitiveComponent Object Reference") (OtherBodyIndex :type Integer) (bFromSweep :type Boolean) (SweepResult :type "HitResult Structure (by ref)"))
  ;[1 1 1 1 30] User Overallaped EndDetection
  (cast `/Game/VRTemplate/Blueprints/VRPawn` OtherActor
    (:`then`
      (if (`self.Recording`)
        ;;[1 1 1] end recording
        (set `self.Recording` false)
        (`self.EndRecordingSession`)
        (`MaterialInstanceDynamic.SetVectorParameterValue` (`self.MatieralIndicator`) "Color" (struct :`R` 0.958333 :`G` 0.120984 :`A` 1.0))
        (`KismetSystemLibrary.PrintString` "ENDDDDDDDDDDDDDDDDDDDDDDDDDDDDDDDDDDDDDDD" true true (struct :`G` 0.66 :`B` 1.0 :`A` 1.0) 5.0)
        (else
          (set `self.ReadyToRecord` true)
          (`MaterialInstanceDynamic.SetVectorParameterValue` (`self.MatieralIndicator`) "Color" (struct :`R` 0.958333 :`G` 0.120984 :`A` 1.0))
          (`KismetSystemLibrary.PrintString` "YAAAAAAAAAAAAAAAAAAAAAAAAAAAAAAAAAAAA" true true (struct :`R` 1.0 :`G` 0.389991 :`A` 1.0) 5.0))))
    (:`CastFailed`
      (`KismetSystemLibrary.PrintString` "EndDetection failed to overlap with VRPawn :(" :!label _label))))

(event `EndRecordingSession`
  ;[0.5121 1 0.3254] Handle Recording Logistics
  ;;[1 1 1] End Recording Session
  (`KismetSystemLibrary.K2_ClearAndInvalidateTimerHandle` (`self.RecorderTimer`))
  (`/Game/_Blueprints/BP_Data.TransmitData` (`self.DataTransmitter`) "stop"))

(event `self.EndDetection.OnComponentEndOverlap`
  (params (OverlappedComponent :type "PrimitiveComponent Object Reference") (OtherActor :type "Actor Object Reference") (OtherComp :type "PrimitiveComponent Object Reference") (OtherBodyIndex :type Integer))
  ;[1 1 1 1 30] User Overallaped EndDetection
  (cast `/Game/VRTemplate/Blueprints/VRPawn` OtherActor
    (:`then`
      (if (`self.ReadyToRecord`)
        ;;[1 1 1] start recording
        (set `self.Recording` true)
        (set `self.ReadyToRecord` false)
        (`self.StartRecordingSession`)
        (`MaterialInstanceDynamic.SetVectorParameterValue` (`self.MatieralIndicator`) "Color" (struct :`G` 0.552832 :`B` 0.958333 :`A` 1.0))
        (`KismetSystemLibrary.PrintString` "SSSSSSSTTTTTTTTARRRRRRRRRRT" true true (struct :`R` 1.0 :`B` 0.563425 :`A` 1.0) 5.0)))
    (:`CastFailed`
      (goto _label))))

(fn `Calibrate`
  (`SceneComponent.K2_SetWorldRotation` (`self.DefaultSceneRoot`) (`SmoothConverters.CalculateRotation` (`self.CalibrationDatapoints`)) false false)
  (`SceneComponent.K2_AddWorldOffset` (`self.DefaultSceneRoot`) (`SmoothConverters.CalculateOffset` (`self.CalibrationDatapoints`) (`SceneComponent.K2_GetComponentLocation` (`self.Calibration1`)) (`SceneComponent.K2_GetComponentLocation` (`self.Calibration2`)) (`SceneComponent.K2_GetComponentLocation` (`self.Calibration3`))) false false))

(fn `DataCollecting`)

(fn `DataToCSV`
  (params (Data :type "_Data Structure"))
  (returns (PrettyData :type String))
  (bind (_time _headpos _controllerleftpos _controllerrightpos _angularacceleration _linearacceleration _angularvelocity _linearvelocity) (break `_Data` Data))
  (return (`KismetStringLibrary.Concat_StrStr` (`KismetStringLibrary.Conv_DoubleToString` _time) "," (`KismetStringLibrary.Conv_VectorToString` _headpos) "," (`KismetStringLibrary.Conv_VectorToString` _controllerleftpos) "," (`KismetStringLibrary.Conv_VectorToString` _controllerrightpos) "," (`KismetStringLibrary.Conv_VectorToString` _angularacceleration) "," (`KismetStringLibrary.Conv_VectorToString` _linearacceleration) "," (`KismetStringLibrary.Conv_VectorToString` _angularvelocity) "," (`KismetStringLibrary.Conv_VectorToString` _linearvelocity))))

(fn `DumpToArray`
  (bind _vrpawnref (`self.VRPawnRef`))
  (bind _locations (`self.Locations`))
  (bind _velocityacc (`self.VelocityAcc`))
  (bind (_headpos _controllerleftpos _controllerrightpos) (`/Game/VRTemplate/Blueprints/VRPawn.GetEverythingData` _vrpawnref))
  (bind (_time_seconds_ _angularacceleration _linearacceleration _angularvelocity _linearvelocity) (`/Game/VRTemplate/Blueprints/VRPawn.GetMovementData` _vrpawnref))
  ;[1 1 1] Location
  (`KismetArrayLibrary.Array_Add` _locations _headpos)
  (`KismetArrayLibrary.Array_Add` _locations _controllerleftpos)
  (`KismetArrayLibrary.Array_Add` _locations _controllerrightpos)
  (`KismetArrayLibrary.Array_Add` _locations (`KismetMathLibrary.MakeVector` _time_seconds_))
  ;[1 1 1] Comment
  (`KismetArrayLibrary.Array_Add` _velocityacc _angularacceleration)
  (`KismetArrayLibrary.Array_Add` _velocityacc _linearacceleration)
  (`KismetArrayLibrary.Array_Add` _velocityacc _angularvelocity)
  (`KismetArrayLibrary.Array_Add` _velocityacc _linearvelocity))

(fn `DumpToStruct`
  (returns (Data :type "_Data Structure"))
  (locals (Data :type "_Data Structure"))
  (bind _vrpawnref (`self.VRPawnRef`))
  (bind (_headpos _controllerleftpos _controllerrightpos) (`/Game/VRTemplate/Blueprints/VRPawn.GetEverythingData` _vrpawnref))
  (bind (_time_seconds_ _angularacceleration _linearacceleration _angularvelocity _linearvelocity) (`/Game/VRTemplate/Blueprints/VRPawn.GetMovementData` _vrpawnref))
  (return (make `_Data` _time_seconds_ _headpos _controllerleftpos _controllerrightpos _angularacceleration _linearacceleration _angularvelocity _linearvelocity)))

(fn `MakeFilename`
  (params (SetName :type String))
  (returns (filename :type String))
  (return (`KismetStringLibrary.Concat_StrStr` (`KismetStringLibrary.Conv_IntToString` (`self.ParticipantID`)) "_situa" (`KismetStringLibrary.Conv_IntToString` (`self.SituationID`)) "_" SetName ".csv")))

(fn `Record`
  (bind _data (`self.DumpToStruct`))
  (bind _prettydata (`self.DataToCSV` _data))
  (`/Game/_Blueprints/BP_Data.TransmitData` (`self.DataTransmitter`) _prettydata))

(fn `SaveData`
  (`|ExecutionSequence`
    (:`then_0`
      (`/Game/_Blueprints/BP_Data.TransmitData` (`self.DataTransmitter`) (`self.FileData` "locations.csv" (`SmoothConverters.VectorArrToString` (`self.Locations`)))))
    (:`then_1`
      (`/Game/_Blueprints/BP_Data.TransmitData` (`self.DataTransmitter`) (`self.FileData` "velociacc.csv" (`SmoothConverters.VectorArrToString` (`self.VelocityAcc`)))))))

(fn `UserConstructionScript`
  (bind _startarea (`self.StartArea`))
  (bind _returnvalue (`PrimitiveComponent.CreateDynamicMaterialInstance` _startarea 0 null "None"))
  (`PrimitiveComponent.SetMaterial` _startarea 0 _returnvalue)
  (set `self.MatieralIndicator` _returnvalue))