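; Touchpoint sphere that shrinks and disappears when something overlaps it, for use attached to a BP_MainProcedure actor.
; On BeginPlay it casts its attach parent to BP_MainProcedure and binds Resetty to that actor's touchpoint reset.
; A DoOnce-guarded overlap deactivates collision and plays a timeline that scales the sphere down, then hides it.
; Resetty restores collision, visibility and scale; the RESETPt function duplicates this logic but is not called here.
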(event `self.ReceiveBeginPlay`
  (bind _returnvalue (`self.GetAttachParentActor`))
  (`/Engine/EditorBlueprintResources/StandardMacros.IsValid` _returnvalue
    (:`Is Valid`
      (bind _asbp_main_procedure (cast `/Game/_Blueprints/BP_MainProcedure` _returnvalue)
        (:`then`
          (bind _output_get (set `self.ProcedureRef` _asbp_main_procedure))
          (add `/Game/_Blueprints/BP_MainProcedure.ResetTouchpoint` _output_get (delegate `Resetty`)))
        (:`CastFailed`
          (`KismetSystemLibrary.PrintString` "BAD CASTING TO MAIN"))))
    (:`Is Not Valid`
      (`KismetSystemLibrary.PrintString` "BAD OWNER "))))

(event `self.Collision.OnComponentBeginOverlap`
  (params (OverlappedComponent :type "PrimitiveComponent Object Reference") (OtherActor :type "Actor Object Reference") (OtherComp :type "PrimitiveComponent Object Reference") (OtherBodyIndex :type Integer) (bFromSweep :type Boolean) (SweepResult :type "HitResult Structure (by ref)"))
  (`/Engine/EditorBlueprintResources/StandardMacros.DoOnce` false :!label _label
    (:`Completed`
      (`ActorComponent.Deactivate` (`self.Collision`))
      (bind (_direction _turnsmall) (`Timeline|Animation` :!via `PlayFromStart`)
        (:`Update`
          ;[1 1 1] Make sphere smaller after intersection
          (`SceneComponent.SetWorldScale3D` (`self.Sphere`) (`KismetMathLibrary.Conv_DoubleToVector` (* _turnsmall 0.16))))
        (:`Finished`
          ;[1 1 1] Set Collision and visiblity both to false
          (`SceneComponent.SetVisibility` (`self.DefaultSceneRoot`) false true)
          (goto _label :!via `Reset`))))))

(event `Resetty`
  (`ActorComponent.Activate` (`self.Collision`) true)
  (`SceneComponent.SetVisibility` (`self.DefaultSceneRoot`) true true)
  (`SceneComponent.SetWorldScale3D` (`self.Sphere`) (`KismetMathLibrary.Conv_DoubleToVector` 0.16)))

(fn `RESETPt`
  (`ActorComponent.Activate` (`self.Collision`) true)
  (`SceneComponent.SetVisibility` (`self.DefaultSceneRoot`) true true)
  (`SceneComponent.SetWorldScale3D` (`self.Sphere`) (`KismetMathLibrary.Conv_DoubleToVector` 0.16)))

(fn `UserConstructionScript`)